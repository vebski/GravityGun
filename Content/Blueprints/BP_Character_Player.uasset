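; BP_Character_Player is the player character Blueprint that handles basic movement, looking and jumping.
; Each Tick reads the MoveForward and MoveRight axes into movement input along the actor's forward and right vectors, then feeds LookRight and LookUp into controller yaw and pitch.
; The Jump action press calls the Character's Jump.
; Input axes are polled on Tick rather than bound to axis events.
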(event `InputAction|Jump`
  (params (Key :type "Key Structure"))
  ;[1 1 1] Movement_Jump
  (:`Pressed`
    (`self.Jump`)))

(event `self.ReceiveTick`
  (params (DeltaSeconds :type "Float (single-precision)"))
  (`|ExecutionSequence`
    (:`then_0`
      ;[1 1 1] Movement_Directions
      (`self.AddMovementInput` (`self.GetActorForwardVector`) (`self.GetInputAxisValue`))
      (`self.AddMovementInput` (`self.GetActorRightVector`) (`self.GetInputAxisValue`)))
    (:`then_1`
      ;[1 1 1] Movement_Rotation
      (`self.AddControllerYawInput` (`self.GetInputAxisValue`))
      (`self.AddControllerPitchInput` (`self.GetInputAxisValue`)))))

(fn `UserConstructionScript`)